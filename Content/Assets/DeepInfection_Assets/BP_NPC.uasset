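; BP_NPC is a talkable NPC built from modular skeletal mesh parts, showing its dialogue one line at a time on screen.
; Each Talk call advances TalkIndex through the Dialogue array, creating the Dialogue_Text_Box widget if it is invalid and updating its text.
; Once the lines run out, the widget is removed from its parent.
; The construction script makes clothing and body meshes follow the pants mesh's pose via leader pose.
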(event `/Game/Assets/DeepInfection_Assets/BP_NPC_Interface.Talk`
  (`/Engine/EditorBlueprintResources/StandardMacros.IncrementInt` (`self.talkIndex`)
    (:`  `
      (if (< (`self.talkIndex`) (`KismetArrayLibrary.Array_Length` (`self.Dialogue`)))
        (`self.UI`
          (:`then`
            _)
          (:`else`
            (bind _returnvalue (`|CreateWidget` "/Game/Assets/DeepInfection_Assets/Dialogue_Text_Box.Dialogue_Text_Box_C" (`GameplayStatics.GetPlayerController` 0)))
            (bind _output_get (set `self.UI` _returnvalue))
            (`UserWidget.AddToViewport` _output_get 0)))
        (`TextBlock.SetText` (`/Game/Assets/DeepInfection_Assets/Dialogue_Text_Box.Talk_Text` (`self.UI`)) (`KismetTextLibrary.Conv_StringToText` (`|GetArrayItem` (`self.Dialogue`) (`self.talkIndex`))))
        (else
          (`Widget.RemoveFromParent` (`self.UI`)))))))

(fn `UserConstructionScript`
  (`SkinnedMeshComponent.SetLeaderPoseComponent` (`self.SK_Man_Shoes`) (`self.SK_Man_Pants`) false false)
  (`SkinnedMeshComponent.SetLeaderPoseComponent` (`self.SK_Man_Head`) (`self.SK_Man_Pants`) false false)
  (`SkinnedMeshComponent.SetLeaderPoseComponent` (`self.SK_Man_Arms`) (`self.SK_Man_Pants`) false false)
  (`SkinnedMeshComponent.SetLeaderPoseComponent` (`self.SK_Man_Bag`) (`self.SK_Man_Pants`) false false)
  (`SkinnedMeshComponent.SetLeaderPoseComponent` (`self.SK_Man_Balaclava`) (`self.SK_Man_Pants`) false false)
  (`SkinnedMeshComponent.SetLeaderPoseComponent` (`self.SK_Man_Pullover`) (`self.SK_Man_Pants`) false false))