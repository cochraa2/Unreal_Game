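; Zombie AI pawn that chases the player survivor on sight and wanders when it sees none.
; PawnSensing sightings of Survivor_BP_Main set CanSeeEnemy and start AIMoveTo toward that survivor; a retriggerable delay clears the flag shortly after sightings stop.
; While the flag is false, Tick feeds a random-length Delay, then moves to a random reachable point nearby.
; The flag is not rechecked after that Delay.
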(event `self.PawnSensing.OnSeePawn`
  (params (Pawn :type "Pawn Object Reference"))
  (bind _assurvivor_bp_main (cast `/Game/Assets/DeepInfection_Assets/Survivor_BP_Main` Pawn))
  (`|ExecutionSequence`
    (:`then_0`
      (set `self.CanSeeEnemy` true)
      (`|AIMoveTo` self (0.0 0.0 0.0) _assurvivor_bp_main))
    (:`then_1`
      (`KismetSystemLibrary.RetriggerableDelay` 0.5)
      (set `self.CanSeeEnemy` false))))

(event `self.ReceiveTick`
  (params (DeltaSeconds :type "Float (single-precision)"))
  (if (not (`self.CanSeeEnemy`))
    (`KismetSystemLibrary.Delay` (`KismetMathLibrary.RandomFloatInRange` 2.0 5.0))
    (`|AIMoveTo` self (`NavigationSystemV1.K2_GetRandomReachablePointInRadius` (`self.K2_GetActorLocation`) 500.0 null null) null)))

(fn `UserConstructionScript`)