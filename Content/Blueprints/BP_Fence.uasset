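; BP_Fence is a procedural fence that lays a straight row of repeated meshes from the actor toward an EndPoint offset.
; The construction script divides the horizontal distance by MeshWidth, rounds it, and adds that many MeshToSpawn components minus the default FenceStart.
; Added pieces attach to FenceStart along its local X axis, so setting its yaw toward the end point turns the whole row, ignoring height.
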(fn `UserConstructionScript`
  (bind _returnvalue (`self.K2_GetActorLocation`))
  (bind _returnvalue_2 (- (`KismetMathLibrary.Round` (/ (`KismetMathLibrary.VSize` (* (`self.End point`) (1.0 1.0 0.0))) (`self.Mesh width`))) 1))
  (`StaticMeshComponent.SetStaticMesh` (`self.Fence start`) (`self.Mesh to spawn`)) ; Change spawned mesh to the new type
  (if (> _returnvalue_2 0)
    (for _index (range 1 (+ _returnvalue_2 1))
      (bind _returnvalue_3 (`AddComponent|NODE_AddStaticMeshComponent-0` :`bManualAttachment` true))
      (`SceneComponent.K2_AttachToComponent` _returnvalue_3 (`self.Fence start`) "None" "KeepWorld" "KeepWorld" "KeepWorld" true)
      (`SceneComponent.K2_SetRelativeLocation` _returnvalue_3 (`KismetMathLibrary.MakeVector` (* _index (`self.Mesh width`))) false false)
      (`StaticMeshComponent.SetStaticMesh` _returnvalue_3 (`self.Mesh to spawn`)) ; Change spawned mesh to the new type
    ))
  (`SceneComponent.K2_SetWorldRotation` (`self.Fence start`) (`KismetMathLibrary.MakeRotator` 0.0 0.0 (.yaw (`KismetMathLibrary.FindLookAtRotation` _returnvalue (+ _returnvalue (`self.End point`))))) false false) ; Rotate the initial mesh to face the end point
)